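; Player character Blueprint for BonedShooter that computes dynamic weapon spread and handles aiming.
; Spread parameters load from a data table, and each tick the locally controlled character triggers a recalculation intended for the server.
; Spread multiplies base, fire and movement factors: firing spikes it before interpolated cooldown, while a velocity threshold drives a timeline through an edge-triggered macro.
; Aiming slows walking and shortens the camera boom via a timeline.
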(event Custom|RecalcSpread
  ;[0.07812 0 1] Calculate spread on server every tick
  (Utilities|FlowControl|Sequence
    (:then_0
      ;;[1 0.1875 0] Shooting spread cooldown
      (Variables|Default|SetFireSpread (Math|Interpolation|FInterpTo (Variables|Default|GetFireSpread) 1.0 (Utilities|Time|GetWorldDeltaSeconds) (Variables|Default|GetFireCooldownSpeed))))
    (:then_1
      (Math|Float|CompareFloat (Math|Vector|VectorLength (Transformation|GetVelocity)) 5e+01
        (:>
          _)
        (:==
          _)
        (:<
          (goto _label Less)))
      ;;[0 1 0.8594] DoOnceInside
      (Utilities|ExecFlipFlop :!label _label
        (:MoreOut
          (bind _spread (Timeline|DynamicSpread Play)
            (:Update
              (Variables|Default|SetMovementSpread (Math|Float|Lerp 1.0 (Variables|Default|GetMovementSpreadMultiplier) _spread)))))
        (:LessOut
          (Timeline|DynamicSpread Reverse))))
    (:then_2
      (CallFunction|RecalculateSpread))))

(event Custom|OnFired_Event_0
  ;[1 0.8438 0] For time saving I didn't care about "RowName Not Found"
  (Variables|Default|SetFireSpread (Variables|Default|GetFireSpreadMultiplier)))

(event EventTick
  (params (DeltaSeconds :type Float%20%28single-precision%29))
  ;[0.07812 0 1] Calculate spread on server every tick
  (|CallParentFunction DeltaSeconds)
  (if (Pawn|IsLocallyControlled)
    (Networking|SwitchHasAuthority
      (:Authority
        (Utilities|FlowControl|Sequence
          (:then_0
            ;;[1 0.1875 0] Shooting spread cooldown
            (Variables|Default|SetFireSpread (Math|Interpolation|FInterpTo (Variables|Default|GetFireSpread) 1.0 (Utilities|Time|GetWorldDeltaSeconds) (Variables|Default|GetFireCooldownSpeed))))
          (:then_1
            (Math|Float|CompareFloat (Math|Vector|VectorLength (Transformation|GetVelocity)) 5e+01
              (:>
                _)
              (:==
                _)
              (:<
                (goto _label Less)))
            ;;[0 1 0.8594] DoOnceInside
            (Utilities|ExecFlipFlop :!label _label
              (:MoreOut
                (bind _spread (Timeline|DynamicSpread Play)
                  (:Update
                    (Variables|Default|SetMovementSpread (Math|Float|Lerp 1.0 (Variables|Default|GetMovementSpreadMultiplier) _spread)))))
              (:LessOut
                (Timeline|DynamicSpread Reverse))))
          (:then_2
            (CallFunction|RecalculateSpread))))
      (:Remote
        (CallFunction|RecalcSpread)))))

(event EventBeginPlay
  ;[1 0.8438 0] For time saving I didn't care about "RowName Not Found"
  (|CallParentFunction)
  (bind _value (Utilities|DataTableExtract "BaseWeaponSpread"))
  (Variables|Default|SetBaseWeaponSpread _value)
  (bind _value_2 (Utilities|DataTableExtract "MovementSpreadMultiplier"))
  (Variables|Default|SetMovementSpreadMultiplier _value_2)
  (bind _value_3 (Utilities|DataTableExtract "FireSpreadMultiplier"))
  (Variables|Default|SetFireSpreadMultiplier _value_3)
  (bind _value_4 (Utilities|DataTableExtract "FireCooldownSpeed"))
  (Variables|Default|SetFireCooldownSpeed _value_4)
  (EventDispatchers|AssignOnFired (delegate Custom|OnFired_Event_0)))

(event EventStartAiming
  ;[0 1 0.8359] Zoom In
  (|CallParentFunction)
  (Variables|/Script/Engine.CharacterMovementComponent|SetMaxWalkSpeed (Variables|Character|GetCharacterMovement) 1e+02)
  (if (Pawn|IsLocallyControlled)
    (bind _aimingalphtrack (Timeline|AimingTimeline Play)
      (:Update
        (Variables|/Script/Engine.SpringArmComponent|SetTargetArmLength (Variables|Default|GetCameraBoom) (Math|Float|Lerp 3e+02 1.5e+02 _aimingalphtrack))))))

(event EventStopAiming
  ;[0 1 0.8359] Zoom In
  (|CallParentFunction)
  (Variables|/Script/Engine.CharacterMovementComponent|SetMaxWalkSpeed (Variables|Character|GetCharacterMovement) 6e+02)
  (if (Pawn|IsLocallyControlled)
    (bind _aimingalphtrack (Timeline|AimingTimeline Reverse)
      (:Update
        (Variables|/Script/Engine.SpringArmComponent|SetTargetArmLength (Variables|Default|GetCameraBoom) (Math|Float|Lerp 3e+02 1.5e+02 _aimingalphtrack))))))

(fn ConstructionScript)

(fn RecalculateSpread
  (Variables|Default|SetCalculatedSpread (* (Variables|Default|GetFireSpread) (Variables|Default|GetMovementSpread) (Variables|Default|GetBaseWeaponSpread))))